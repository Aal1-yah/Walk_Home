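; Player character with walk, jump, glide and dash, using Enhanced Input through a mapping context added at BeginPlay.
; Walking moves along world X at a fixed max speed.
; Holding jump past the apex starts a glide with low gravity and high air control, reset on release or landing.
; Dash launches the character horizontally at a multiple of its current velocity, gated by a flag that clears after a one-second delay.
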(event Custom|OnApexReached
  (bind _charactermovement (Variables|Character|GetCharacterMovement))
  ;[0.15 0.15 0.15 0.5] Character Floats
  (Variables|/Script/Engine.CharacterMovementComponent|SetGravityScale _charactermovement 0.1)
  (Variables|/Script/Engine.CharacterMovementComponent|SetAirControl _charactermovement 0.8))

(event Input|EnhancedActionEvents|EnhancedInputActionIA_Jump
  (params (ActionValue :type Boolean) (ElapsedSeconds :type Float%20%28double-precision%29) (TriggeredSeconds :type Float%20%28double-precision%29) (InputAction :type Input%20Action%20Object%20Reference :default "/Game/Inputs/IA_Jump.IA_Jump"))
  (bind _charactermovement (Variables|Character|GetCharacterMovement))
  (bind _charactermovement_2 (Variables|Character|GetCharacterMovement))
  ;[0.15 0.15 0.15 0.5] Character Jump
  (:Started
    (Character|Jump)
    ;[0.15 0.15 0.15 0.5] Checks if jumping
    (Variables|/Script/Engine.CharacterMovementComponent|SetbNotifyApex _charactermovement true)
    ;[0.15 0.15 0.15 0.5] Character Glides when holding space
    (Character|BindEventtoOnReachedJumpApex (EventDispatchers|CreateEvent :!event Custom|OnApexReached)))
  (:Completed
    (Character|StopJumping)
    (Variables|/Script/Engine.CharacterMovementComponent|SetbNotifyApex _charactermovement false)
    (EventDispatchers|UnbindallEventsfromOnReachedJumpApex)
    (Variables|/Script/Engine.CharacterMovementComponent|SetGravityScale _charactermovement_2 1.0)
    (Variables|/Script/Engine.CharacterMovementComponent|SetAirControl _charactermovement_2 0.05)))

(event Input|EnhancedActionEvents|EnhancedInputActionIA_Walk
  (params (ActionValue :type Float%20%28double-precision%29) (ElapsedSeconds :type Float%20%28double-precision%29) (TriggeredSeconds :type Float%20%28double-precision%29) (InputAction :type Input%20Action%20Object%20Reference :default "/Game/Inputs/IA_Walk.IA_Walk"))
  ;[0.15 0.15 0.15 0.5] Walk Speed
  (Variables|/Script/Engine.CharacterMovementComponent|SetMaxWalkSpeed (Variables|Character|GetCharacterMovement) 2e+02)
  (Pawn|Input|AddMovementInput "1.000000,0.000000,0.000000" ActionValue false))

(event Input|EnhancedActionEvents|EnhancedInputActionIA_Dash
  (params (ActionValue :type Boolean) (ElapsedSeconds :type Float%20%28double-precision%29) (TriggeredSeconds :type Float%20%28double-precision%29) (InputAction :type Input%20Action%20Object%20Reference :default "/Game/Inputs/IA_Dash.IA_Dash"))
  (bind _returnvalue (Transformation|GetVelocity))
  (bind _returnvalue_2 (* _returnvalue 1e+01))
  ;[0.15 0.15 0.15 0.5] Checks if dashing
  (if (not (Variables|Default|GetIsDashing))
    (Variables|Default|SetIsDashing true)
    (Character|LaunchCharacter (Math|Vector|MakeVector (.x _returnvalue_2) (.y _returnvalue_2) 0.0) false false)
    (Utilities|FlowControl|Delay 1.0)
    (Variables|Default|SetIsDashing false)))

(event EventBeginPlay
  (Input|AddMappingContext (PlayerController|LocalPlayerSubsystems|GetEnhancedInputLocalPlayerSubsystem (Game|GetPlayerController 0)) "/Game/Inputs/IMC_PaperPlayer.IMC_PaperPlayer" 0 "(bIgnoreAllPressedKeysUntilRelease=True,bForceImmediately=False,bNotifyUserSettings=False)"))

(event Collision|EventActorBeginOverlap
  (params (OtherActor :type Actor%20Object%20Reference)))

(event EventTick
  (params (DeltaSeconds :type Float%20%28single-precision%29)))

(event EventOnLanded
  (params (Hit :type Hit%20Result%20Structure%20%28by%20ref%29))
  (bind _charactermovement (Variables|Character|GetCharacterMovement))
  ;[0.15 0.15 0.15 0.5] Gravity returns to normal once landed
  (Variables|/Script/Engine.CharacterMovementComponent|SetGravityScale _charactermovement 1.0)
  (Variables|/Script/Engine.CharacterMovementComponent|SetAirControl _charactermovement 0.05))

(fn ConstructionScript)